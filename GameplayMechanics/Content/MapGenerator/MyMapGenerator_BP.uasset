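; Map generator actor that exposes Poisson disk sampling, Delaunay triangulation and path generation as separately callable steps.
; On BeginPlay it creates a MapGeneratorWidget_BP, registers itself as owner and fills it with the current seed, grid extent, sphere radius, iteration and sample settings.
; MapValueChangedEvent copies the widget's values back into those settings without regenerating.
; Each Execute function is a thin wrapper around a generation routine defined outside this graph.
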(event `self.ReceiveBeginPlay`
  (bind _returnvalue (`|CreateWidget` "/Game/MapGenerator/MapGeneratorWidget_BP.MapGeneratorWidget_BP_C" (`GameplayStatics.GetPlayerController` 0)))
  (bind _output_get (set `self.MapWidget` _returnvalue))
  (`UserWidget.AddToViewport` _output_get 0)
  (set `/Game/MapGenerator/MapGeneratorWidget_BP.Owner` self (`self.MapWidget`))
  (`/Game/MapGenerator/MapGeneratorWidget_BP.UpdateValues` (`self.MapWidget`) (`self.Seed`) (`self.GridExtend`) (`self.SphereRadius`) (`self.Iterations`) (`self.NumSampleBeforeRejection`)))

(event `MapValueChangedEvent`
  (bind _mapwidget (`self.MapWidget`))
  (set `self.Seed` (`/Game/MapGenerator/MapGeneratorWidget_BP.SeedValue` _mapwidget))
  (set `self.GridExtend` (`/Game/MapGenerator/MapGeneratorWidget_BP.GridValue` _mapwidget))
  (set `self.SphereRadius` (`/Game/MapGenerator/MapGeneratorWidget_BP.SphereValue` _mapwidget))
  (set `self.Iterations` (`/Game/MapGenerator/MapGeneratorWidget_BP.IterationsValue` _mapwidget))
  (set `self.NumSampleBeforeRejection` (`/Game/MapGenerator/MapGeneratorWidget_BP.SamplesValue` _mapwidget)))

(fn `ExecuteDelaunary`
  (`self.DelaunaryTriangulation`))

(fn `ExecuteGeneratePath`
  (`self.GeneratePaths`))

(fn `ExecutePosionDisk`
  (`self.MyPoisonDiskSamplingAlgorithm`))

(fn `UserConstructionScript`)